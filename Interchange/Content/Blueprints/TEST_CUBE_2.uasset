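; TEST_CUBE_2 is a test actor that spawns and removes TEST_CUBE actors in response to MBAP success and failure events.
; MBAPonSuccess spawns a cube with fixed rotation and scale at a random offset around its own location, storing it in TEMPBOX.
; MBAPonFailure destroys the actor held in TEMPBOX, which is only the most recent spawn, as each success overwrites that reference.
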(event EventBeginPlay)

(event Collision|EventActorBeginOverlap
  (params (OtherActor :type Actor%20Object%20Reference)))

(event EventTick
  (params (DeltaSeconds :type Float%20%28single-precision%29)))

(event EventMBAPonSuccess
  (bind _returnvalue (Game|SpawnActorfromClass "/Game/Blueprints/TEST_CUBE.TEST_CUBE_C" (Math|Transform|MakeTransform (+ (Transformation|GetActorLocation) (Math|Vector|MakeVector (Math|Random|RandomFloatinRange -2e+02 2e+02) (Math|Random|RandomFloatinRange -2e+02 2e+02) (Math|Random|RandomFloatinRange -2e+02 3e+02))) "50.000000,77.000000,20.000000") "Undefined" 0 0))
  (Variables|Default|SetTEMPBOX _returnvalue))

(event EventMBAPonFailure
  (Actor|DestroyActor (Variables|Default|GetTEMPBOX)))

(fn ConstructionScript)