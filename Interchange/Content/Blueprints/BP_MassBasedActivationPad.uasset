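; A pressure pad actor that activates when the total mass resting on it reaches TargetMass.
; Trigger overlap events add and subtract each component's mass from CurrentTotalPressure, which Tick compares against the target.
; On each state change, it swaps the Pad's on/off material and sends MBAPOnSuccessMessage or MBAPOnFailureMessage to every entry in ExecutableObjects.
; Activation also prints a debug string.
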(event OnComponentBeginOverlap(Trigger)
  (params (OverlappedComponent :type Primitive%20Component%20Object%20Reference) (OtherActor :type Actor%20Object%20Reference) (OtherComp :type Primitive%20Component%20Object%20Reference) (OtherBodyIndex :type Integer) (bFromSweep :type Boolean) (SweepResult :type Hit%20Result%20Structure%20%28by%20ref%29))
  (Variables|Default|SetCurrentTotalPressure (+ (Physics|GetMass OtherComp) (Variables|Default|GetCurrentTotalPressure))))

(event OnComponentEndOverlap(Trigger)
  (params (OverlappedComponent :type Primitive%20Component%20Object%20Reference) (OtherActor :type Actor%20Object%20Reference) (OtherComp :type Primitive%20Component%20Object%20Reference) (OtherBodyIndex :type Integer))
  (Variables|Default|SetCurrentTotalPressure (- (Variables|Default|GetCurrentTotalPressure) (Physics|GetMass OtherComp))))

(event EventBeginPlay)

(event EventTick
  (params (DeltaSeconds :type Float%20%28single-precision%29))
  (bind _pad (Variables|Default|GetPad))
  (if (>= (Variables|Default|GetCurrentTotalPressure) (Variables|Default|GetTargetMass))
    (if (== (Variables|Default|GetIsActivated) false)
      (Variables|Default|SetIsActivated true)
      (Rendering|Material|SetMaterial _pad 0 "/Game/Materials/M_MBAP_On.M_MBAP_On")
      (for _array_element (Variables|Default|GetExecutableObjects)
        (Class|BPMBAPExecutionInterface|MBAPonSuccess(Message) _array_element))
      (Development|PrintString "YAY" true true "(R=1.000000,G=0.988650,B=0.187166,A=1.000000)"))
    (elif (not (== (Variables|Default|GetIsActivated) false))
      (Variables|Default|SetIsActivated false)
      (Rendering|Material|SetMaterial _pad 0 "/Game/Materials/M_MBAP_Off.M_MBAP_Off")
      (for _array_element_2 (Variables|Default|GetExecutableObjects)
        (Class|BPMBAPExecutionInterface|MBAPonFailure(Message) _array_element_2)))))

(fn ConstructionScript)