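; First-person character Blueprint that adds a mantle check for climbing onto ledges; its event graph is empty.
; Mantle chains a forward capsule trace, a vertical sphere trace for a walkable surface and CheckMantleRoom for clearance.
; On success it disables movement and returns a raised target location, without moving the character itself.
; CheckMantleRoom can crouch in limited space; an unfinished camera shake is left unconnected.
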(event EventBeginPlay)

(event Collision|EventActorBeginOverlap
  (params (OtherActor :type Actor%20Object%20Reference)))

(event EventTick
  (params (DeltaSeconds :type Float%20%28single-precision%29)))

(fn ConstructionScript)

(fn Mantle
  (bind _returnvalue (Transformation|GetActorLocation))
  (bind _returnvalue_2 (+ _returnvalue "0,0,45.000000"))
  (Utilities|FlowControl|Sequence
    (:then_0
      ;[1 0.8035 0.9083] Check for blocking wall.
      (bind _outhit (Collision|CapsuleTraceByChannel _returnvalue_2 (+ _returnvalue_2 (* (Transformation|GetActorForwardVector) "30.000000,30.000000,30.000000")) 34.0 88.0 "TraceTypeQuery1" false 0 "None"))
      (if (Math|Boolean|ANDBoolean (not (Class|CharacterMovementComponent|IsWalkable (Variables|Character|GetCharacterMovement) _outhit)) (not (.bBlockingHit (Collision|BreakHitResult _outhit))) (not (.bInitialOverlap (Collision|BreakHitResult _outhit))))
        (LocalVariables|SetInitPoint (.ImpactPoint (Collision|BreakHitResult _outhit)))
        (LocalVariables|SetInitNormal (.ImpactNormal (Collision|BreakHitResult _outhit)))
        (else
          (return false "0, 0, 0"))))
    (:then_1
      ;[0.6963 0.8433 1] Trace downward.
      (bind _outhit_2 (Collision|SphereTraceByChannel (+ (+ (Math|Vector|MakeVector (.x (LocalVariables|GetInitPoint)) (.y (LocalVariables|GetInitPoint)) (- (.z (Transformation|GetActorLocation)) 45.0)) (* (LocalVariables|GetInitNormal) -3e+01)) "0,0,-120.000000") (+ (Math|Vector|MakeVector (.x (LocalVariables|GetInitPoint)) (.y (LocalVariables|GetInitPoint)) (- (.z (Transformation|GetActorLocation)) 45.0)) (* (LocalVariables|GetInitNormal) -3e+01)) 34.0 "TraceTypeQuery1" false 0 "None"))
      (if (and (.bBlockingHit (Collision|BreakHitResult _outhit_2)) (Class|CharacterMovementComponent|IsWalkable (Variables|Character|GetCharacterMovement) _outhit_2))
        (LocalVariables|SetTargetLoc (.Location (Collision|BreakHitResult _outhit_2)))
        (else
          (return false "0, 0, 0"))))
    (:then_2
      ;[0.7231 1 0.7157] Check room & mantle
      (bind _hasroom (CallFunction|CheckMantleRoom (LocalVariables|GetTargetLoc)))
      (if _hasroom
        (Pawn|Components|CharacterMovement|SetMovementMode (Variables|Character|GetCharacterMovement) "MOVE_None" 0)
        (return true (Math|Vector|MakeVector (.x (LocalVariables|GetTargetLoc)) (.y (LocalVariables|GetTargetLoc)) (+ (.z (LocalVariables|GetTargetLoc)) (* (Components|Capsule|GetUnscaledCapsuleHalfHeight (Variables|Default|GetCapsuleComponent)) 0.5))))))))

(fn CheckMantleRoom
  (params (TargetLoc :type Vector))
  (bind _capsulecomponent (Variables|Default|GetCapsuleComponent))
  (bind _returnvalue (Components|Capsule|GetScaledCapsuleHalfHeight _capsulecomponent))
  (bind _outhit (Collision|SphereTraceByChannel (Math|Vector|MakeVector (.x TargetLoc) (.y TargetLoc) (+ (.z TargetLoc) 15.0)) (Math|Vector|MakeVector (.x TargetLoc) (.y TargetLoc) (+ (.z TargetLoc) (Components|Capsule|GetScaledCapsuleRadius _capsulecomponent))) _returnvalue "TraceTypeQuery1" false 0 "None"))
  (if (Math|Boolean|NORBoolean (.bBlockingHit (Collision|BreakHitResult _outhit)) (.bInitialOverlap (Collision|BreakHitResult _outhit)))
    (return true)
    (elif (<= (.Distance (Collision|BreakHitResult _outhit)) (* _returnvalue 0.5))
      (return false)
      (else
        (Character|Crouch)))))